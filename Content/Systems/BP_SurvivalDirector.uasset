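; Survival director that runs the player's suit resources, clone respawn and save progress.
; Tick integrates oxygen, power, integrity and stamina from habitat, storm and movement state, driving walk speed, spotlight shutoff and oxygen warnings.
; Empty oxygen or integrity respawns a clone, moving carried scrap into a recovery crate at the death spot, reclaimed with E.
; Progress persists to a version-checked save slot via timed autosave, respawn, crate recovery and F5, loading on BeginPlay or F9.
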(event `self.ReceiveBeginPlay`
  (`self.EnableInput` (`GameplayStatics.GetPlayerController` 0))
  (`self.LoadProgress`)
  (`self.RefreshRecoveryCache`))

(event `Key|E` :consume false
  (params (Key :type "Key Structure"))
  (:`Pressed`
    (`self.RecoverCrate`)))

(event `Key|F5` :consume false
  (params (Key :type "Key Structure"))
  (:`Pressed`
    (`self.SaveProgress`)))

(event `Key|F9` :consume false
  (params (Key :type "Key Structure"))
  (:`Pressed`
    (`self.LoadProgress`)))

(event `self.ReceiveTick`
  (params (DeltaSeconds :type "Float (single-precision)"))
  (bind _returnvalue (`GameplayStatics.GetPlayerCharacter` 0))
  (bind _returnvalue_2 (+ (`self.SaveElapsed`) DeltaSeconds))
  (bind _returnvalue_3 (+ (`self.WarningElapsed`) DeltaSeconds))
  (bind _returnvalue_4 (`DustfallSurvivalLibrary.IsWithinHabitat` (`self.K2_GetActorLocation` (`GameplayStatics.GetPlayerCharacter` 0)) (`self.HabitatCenter`) (`self.HabitatHalfExtent`)))
  (bind _returnvalue_5 (`DustfallSurvivalLibrary.UpdateSprintExhaustion` (`self.Stamina`) (`self.StaminaBeforeTick`) (`self.SprintExhausted`) (`/Game/Data/BP_SurvivalData.StaminaRecoveryThreshold` (`self.Tuning`))))
  (set `self.InHabitat` _returnvalue_4)
  (set `self.Oxygen` (`DustfallSurvivalLibrary.IntegrateResource` (`self.Oxygen`) (`KismetMathLibrary.SelectFloat` (`/Game/Data/BP_SurvivalData.OxygenRefillPerSecond` (`self.Tuning`)) (* (`/Game/Data/BP_SurvivalData.OxygenDrainPerSecond` (`self.Tuning`)) -1.0) _returnvalue_4) DeltaSeconds (`/Game/Data/BP_SurvivalData.MaxOxygen` (`self.Tuning`))))
  (set `self.Power` (`DustfallSurvivalLibrary.IntegrateResource` (`self.Power`) (`KismetMathLibrary.SelectFloat` (`/Game/Data/BP_SurvivalData.PowerRefillPerSecond` (`self.Tuning`)) (* (`/Game/Data/BP_SurvivalData.PowerDrainPerSecond` (`self.Tuning`)) -1.0) _returnvalue_4) DeltaSeconds (`/Game/Data/BP_SurvivalData.MaxPower` (`self.Tuning`))))
  (set `self.Integrity` (`DustfallSurvivalLibrary.IntegrateResource` (`self.Integrity`) (`KismetMathLibrary.SelectFloat` 0.0 (* (* (`/Game/World/Blueprints/BP_DustfallEnvironmentDirector.StormIntensity` (`self.EnvironmentDirector`)) (`/Game/Data/BP_SurvivalData.StormIntegrityDrainPerSecond` (`self.Tuning`))) -1.0) _returnvalue_4) DeltaSeconds (`/Game/Data/BP_SurvivalData.MaxIntegrity` (`self.Tuning`))))
  (set `self.StaminaBeforeTick` (`self.Stamina`))
  (set `self.Stamina` (`DustfallSurvivalLibrary.IntegrateResource` (`self.Stamina`) (`KismetMathLibrary.SelectFloat` (* (`/Game/Data/BP_SurvivalData.StaminaDrainPerSecond` (`self.Tuning`)) -1.0) (`/Game/Data/BP_SurvivalData.StaminaRefillPerSecond` (`self.Tuning`)) (> (`KismetMathLibrary.VSizeXY` (`self.GetVelocity` _returnvalue)) (`/Game/Data/BP_SurvivalData.SprintVelocityThreshold` (`self.Tuning`)))) DeltaSeconds (`/Game/Data/BP_SurvivalData.MaxStamina` (`self.Tuning`))))
  (set `self.SprintExhausted` _returnvalue_5)
  (set `CharacterMovementComponent.MaxWalkSpeed` (`KismetMathLibrary.SelectFloat` (`/Game/Data/BP_SurvivalData.ExhaustedSpeed` (`self.Tuning`)) (`KismetMathLibrary.SelectFloat` (`/Game/Data/BP_SurvivalData.SprintSpeed` (`self.Tuning`)) (`/Game/Data/BP_SurvivalData.WalkSpeed` (`self.Tuning`)) (or (`PlayerController.IsInputKeyDown` (`GameplayStatics.GetPlayerController` 0) "(") (`self.SprintRequested`))) _returnvalue_5) (`Character.CharacterMovement` _returnvalue))
  (if (<= (`self.Power`) 0.0)
    (`SceneComponent.SetVisibility` (`self.GetComponentByClass` _returnvalue "/Script/Engine.SpotLightComponent") false false))
  (if (or (<= (`self.Oxygen`) 0.0) (<= (`self.Integrity`) 0.0))
    (`self.RespawnClone`)
    (else
      (set `self.SaveElapsed` _returnvalue_2)
      (if (>= _returnvalue_2 (`/Game/Data/BP_SurvivalData.SaveIntervalSeconds` (`self.Tuning`)))
        (set `self.SaveElapsed` 0.0)
        (`self.SaveProgress`))
      (set `self.WarningElapsed` _returnvalue_3)
      (if (and (<= (`self.Oxygen`) (`/Game/Data/BP_SurvivalData.OxygenWarningThreshold` (`self.Tuning`))) (>= _returnvalue_3 (`/Game/Data/BP_SurvivalData.OxygenWarningCooldown` (`self.Tuning`))))
        (`GameplayStatics.PlaySound2D` "/Game/Audio/Suit/S_OxygenWarning_Phase3.S_OxygenWarning_Phase3" 0.65 1.0 0.0 null null)
        (set `self.WarningElapsed` 0.0)
        (set `self.OxygenWarningCount` (+ (`self.OxygenWarningCount`) 1))))))

(fn `GetSuitState`
  (returns (Oxygen :type "Float (double-precision)") (Power :type "Float (double-precision)") (Integrity :type "Float (double-precision)") (Stamina :type "Float (double-precision)") (CloneGeneration :type Integer))
  (return (`self.Oxygen`) (`self.Power`) (`self.Integrity`) (`self.Stamina`) (`self.CloneGeneration`)))

(fn `LoadProgress`
  (bind _returnvalue (`GameplayStatics.DoesSaveGameExist` (`self.SaveSlotName`)))
  (if _returnvalue
    (bind _returnvalue_2 (`GameplayStatics.LoadGameFromSlot` (`self.SaveSlotName`)))
    (bind _asbp_dustfall_save_game (cast `/Game/Systems/BP_DustfallSaveGame` _returnvalue_2))
    (if (== (`/Game/Systems/BP_DustfallSaveGame.SaveVersion` _asbp_dustfall_save_game) 1)
      (set `self.Oxygen` (`/Game/Systems/BP_DustfallSaveGame.Oxygen` _asbp_dustfall_save_game))
      (set `self.Power` (`/Game/Systems/BP_DustfallSaveGame.Power` _asbp_dustfall_save_game))
      (set `self.Integrity` (`/Game/Systems/BP_DustfallSaveGame.Integrity` _asbp_dustfall_save_game))
      (set `self.Stamina` (`/Game/Systems/BP_DustfallSaveGame.Stamina` _asbp_dustfall_save_game))
      (set `self.CloneGeneration` (`/Game/Systems/BP_DustfallSaveGame.CloneGeneration` _asbp_dustfall_save_game))
      (set `self.CarriedScrap` (`/Game/Systems/BP_DustfallSaveGame.CarriedScrap` _asbp_dustfall_save_game))
      (set `self.CrateScrap` (`/Game/Systems/BP_DustfallSaveGame.CrateScrap` _asbp_dustfall_save_game))
      (set `self.CrateActive` (`/Game/Systems/BP_DustfallSaveGame.CrateActive` _asbp_dustfall_save_game))
      (set `self.CrateLocation` (`/Game/Systems/BP_DustfallSaveGame.CrateLocation` _asbp_dustfall_save_game))
      (set `self.SavedLocation` (`/Game/Systems/BP_DustfallSaveGame.SavedLocation` _asbp_dustfall_save_game))
      (`self.K2_SetActorLocation` (`GameplayStatics.GetPlayerCharacter` 0) (`self.SavedLocation`) false true)
      (`self.RefreshRecoveryCache`))))

(fn `RecoverCrate`
  (if (`self.CrateActive`)
    (if (<= (`KismetMathLibrary.Vector_Distance` (`self.K2_GetActorLocation` (`GameplayStatics.GetPlayerCharacter` 0)) (`self.CrateLocation`)) (`/Game/Data/BP_SurvivalData.RecoveryDistance` (`self.Tuning`)))
      (set `self.CarriedScrap` (+ (`self.CarriedScrap`) (`self.CrateScrap`)))
      (set `self.CrateScrap` 0)
      (set `self.CrateActive` false)
      (`self.RefreshRecoveryCache`)
      (`self.SaveProgress`))))

(fn `RefreshRecoveryCache`
  (bind _recoveryactor (`self.RecoveryActor`))
  (`self.SetActorHiddenInGame` _recoveryactor (not (`self.CrateActive`)))
  (`self.K2_SetActorLocation` _recoveryactor (`self.CrateLocation`) false true))

(fn `RespawnClone`
  (if (not (`self.DeathInProgress`))
    (set `self.DeathInProgress` true)
    (set `self.CrateLocation` (+ (`self.K2_GetActorLocation` (`GameplayStatics.GetPlayerCharacter` 0)) (0.0 0.0 -65.0)))
    (set `self.CrateScrap` (+ (`self.CrateScrap`) (`self.CarriedScrap`)))
    (set `self.CarriedScrap` 0)
    (set `self.CrateActive` true)
    (set `self.CloneGeneration` (+ (`self.CloneGeneration`) 1))
    (set `self.Oxygen` (`/Game/Data/BP_SurvivalData.MaxOxygen` (`self.Tuning`)))
    (set `self.Power` (`/Game/Data/BP_SurvivalData.MaxPower` (`self.Tuning`)))
    (set `self.Integrity` (`/Game/Data/BP_SurvivalData.MaxIntegrity` (`self.Tuning`)))
    (set `self.Stamina` (`/Game/Data/BP_SurvivalData.MaxStamina` (`self.Tuning`)))
    (set `self.SprintExhausted` false)
    (`self.K2_SetActorLocation` (`GameplayStatics.GetPlayerCharacter` 0) (`self.CloneSpawn`) false true)
    (set `self.DeathInProgress` false)
    (`self.RefreshRecoveryCache`)
    (`self.SaveProgress`)))

(fn `SaveProgress`
  (set `self.SavedLocation` (`self.K2_GetActorLocation` (`GameplayStatics.GetPlayerCharacter` 0)))
  (bind _returnvalue (`GameplayStatics.CreateSaveGameObject` "/Game/Systems/BP_DustfallSaveGame.BP_DustfallSaveGame_C"))
  (bind _asbp_dustfall_save_game (cast `/Game/Systems/BP_DustfallSaveGame` _returnvalue))
  (set `/Game/Systems/BP_DustfallSaveGame.Oxygen` (`self.Oxygen`) _asbp_dustfall_save_game)
  (set `/Game/Systems/BP_DustfallSaveGame.Power` (`self.Power`) _asbp_dustfall_save_game)
  (set `/Game/Systems/BP_DustfallSaveGame.Integrity` (`self.Integrity`) _asbp_dustfall_save_game)
  (set `/Game/Systems/BP_DustfallSaveGame.Stamina` (`self.Stamina`) _asbp_dustfall_save_game)
  (set `/Game/Systems/BP_DustfallSaveGame.CloneGeneration` (`self.CloneGeneration`) _asbp_dustfall_save_game)
  (set `/Game/Systems/BP_DustfallSaveGame.CarriedScrap` (`self.CarriedScrap`) _asbp_dustfall_save_game)
  (set `/Game/Systems/BP_DustfallSaveGame.CrateScrap` (`self.CrateScrap`) _asbp_dustfall_save_game)
  (set `/Game/Systems/BP_DustfallSaveGame.CrateActive` (`self.CrateActive`) _asbp_dustfall_save_game)
  (set `/Game/Systems/BP_DustfallSaveGame.CrateLocation` (`self.CrateLocation`) _asbp_dustfall_save_game)
  (set `/Game/Systems/BP_DustfallSaveGame.SavedLocation` (`self.SavedLocation`) _asbp_dustfall_save_game)
  (set `/Game/Systems/BP_DustfallSaveGame.SaveVersion` 1 _asbp_dustfall_save_game)
  (bind _returnvalue_2 (`GameplayStatics.SaveGameToSlot` _asbp_dustfall_save_game (`self.SaveSlotName`)))
  (set `self.LastSaveSucceeded` _returnvalue_2))

(fn `UserConstructionScript`)