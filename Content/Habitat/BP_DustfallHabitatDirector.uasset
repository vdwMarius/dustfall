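; Habitat director that runs a two-door airlock cycle when a nearby player presses E or DF_RequestAirlock fires.
; The player's side of the airlock sets travel direction, so the near door opens first, closes, then the far door opens and closes.
; Tick drives both doors from one timer by teleporting them between raised and lowered heights.
; The timer pauses while the player stands in a doorway about to close.
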(event `self.ReceiveBeginPlay`
  (`self.EnableInput` (`GameplayStatics.GetPlayerController` 0)))

(event `Key|E` :consume false
  (params (Key :type "Key Structure"))
  (bind _returnvalue (- (`self.K2_GetActorLocation` (`GameplayStatics.GetPlayerPawn` 0)) (`self.HabitatOrigin`)))
  (:`Pressed`
    (if (and (< (`KismetMathLibrary.VSize` _returnvalue) 1500.0) (not (`self.Cycling`)))
      (set `self.TravelOut` (< (.x _returnvalue) 750.0) :!label _label)
      (set `self.CycleTime` 0.0)
      (set `self.Cycling` true))))

(event `DF_RequestAirlock`
  (if (and (< (`KismetMathLibrary.VSize` (- (`self.K2_GetActorLocation` (`GameplayStatics.GetPlayerPawn` 0)) (`self.HabitatOrigin`))) 1500.0) (not (`self.Cycling`)))
    (goto _label)))

(event `self.ReceiveTick`
  (params (DeltaSeconds :type "Float (single-precision)"))
  (bind _cycletime (`self.CycleTime`))
  (bind _cycling (`self.Cycling`))
  (bind _travelout (`self.TravelOut`))
  (bind _habitatorigin (`self.HabitatOrigin`))
  (bind _returnvalue (< _cycletime 4.0))
  (bind _returnvalue_2 (and (> _cycletime 6.0) (< _cycletime 10.0)))
  (bind _x (.x (- (`self.K2_GetActorLocation` (`GameplayStatics.GetPlayerPawn` 0)) _habitatorigin)))
  (bind _returnvalue_3 (< (`KismetMathLibrary.Abs` (.y (- (`self.K2_GetActorLocation` (`GameplayStatics.GetPlayerPawn` 0)) _habitatorigin))) 145.0))
  (set `self.CycleTime` (`KismetMathLibrary.SelectFloat` (`KismetMathLibrary.SelectFloat` _cycletime (+ _cycletime DeltaSeconds) (or (and (and (>= _cycletime 3.0) (< _cycletime 4.0)) (and (< (`KismetMathLibrary.Abs` (- _x (`KismetMathLibrary.SelectFloat` 500.0 1000.0 (`self.TravelOut`)))) 95.0) _returnvalue_3)) (and (and (>= _cycletime 9.0) (< _cycletime 10.0)) (and (< (`KismetMathLibrary.Abs` (- _x (`KismetMathLibrary.SelectFloat` 1000.0 500.0 (`self.TravelOut`)))) 95.0) _returnvalue_3)))) 0.0 _cycling))
  (set `self.Cycling` (and _cycling (not (>= _cycletime 12.0))))
  (`self.K2_SetActorLocation` (`self.InnerDoor`) (+ (`KismetMathLibrary.MakeVector` 500.0 0.0 (+ (`KismetMathLibrary.SelectFloat` (`KismetMathLibrary.SelectFloat` (`KismetMathLibrary.SelectFloat` 350.0 0.0 _returnvalue) (`KismetMathLibrary.SelectFloat` 350.0 0.0 _returnvalue_2) _travelout) 0.0 _cycling) 190.0)) _habitatorigin) false true)
  (`self.K2_SetActorLocation` (`self.OuterDoor`) (+ (`KismetMathLibrary.MakeVector` 1000.0 0.0 (+ (`KismetMathLibrary.SelectFloat` (`KismetMathLibrary.SelectFloat` (`KismetMathLibrary.SelectFloat` 350.0 0.0 _returnvalue_2) (`KismetMathLibrary.SelectFloat` 350.0 0.0 _returnvalue) _travelout) 0.0 _cycling) 190.0)) _habitatorigin) false true))

(fn `UserConstructionScript`)