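; Environment director for Dustfall that runs the day-night cycle and dust weather from an EnvironmentData asset.
; Each Tick advances time of day and a timed calm, haze, storm, haze weather loop.
; Cosine-based daylight and smoothly interpolated storm intensity drive sun, sky light, fog and wind volume, then an environment-changed event fires every frame.
; Functions allow overriding weather or time and reading current state.
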(event `self.ReceiveTick`
  (params (DeltaSeconds :type "Float (single-precision)"))
  (bind _fogcomponent (`self.FogComponent`))
  (bind _suncomponent (`self.SunComponent`))
  (bind _weather (`self.Weather`))
  (bind _returnvalue (>= _weather 1))
  (bind _returnvalue_2 (>= _weather 2))
  (bind _weatherblendspeed (`/Game/Data/BP_EnvironmentPhase2Data.WeatherBlendSpeed` (`self.EnvironmentData`)))
  (bind _returnvalue_3 (`KismetMathLibrary.Lerp` 1.0 (`/Game/Data/BP_EnvironmentPhase2Data.StormLightMultiplier` (`self.EnvironmentData`)) (`self.StormIntensity`)))
  (bind _output_get (set `self.WeatherElapsed` (+ (`self.WeatherElapsed`) DeltaSeconds)))
  (if (>= _output_get (`KismetMathLibrary.SelectFloat` (`/Game/Data/BP_EnvironmentPhase2Data.StormDuration` (`self.EnvironmentData`)) (`KismetMathLibrary.SelectFloat` (`/Game/Data/BP_EnvironmentPhase2Data.HazeDuration` (`self.EnvironmentData`)) (`/Game/Data/BP_EnvironmentPhase2Data.CalmDuration` (`self.EnvironmentData`)) _returnvalue) _returnvalue_2))
    (set `self.WeatherElapsed` 0.0)
    (bind _output_get_2 (set `self.WeatherStage` (mod (+ (`self.WeatherStage`) 1) 4)))
    (set `self.Weather` (`KismetMathLibrary.SelectInt` 1 _output_get_2 (>= _output_get_2 3))))
  (bind _output_get_3 (set `self.TimeOfDay` (`KismetMathLibrary.FMod` (+ (`self.TimeOfDay`) (/ DeltaSeconds (`KismetMathLibrary.FMax` (`/Game/Data/BP_EnvironmentPhase2Data.DayLengthSeconds` (`self.EnvironmentData`)) 1.0))) 1.0)))
  (bind _returnvalue_4 (`KismetMathLibrary.DegCos` (* _output_get_3 360.0)))
  (`SceneComponent.K2_SetWorldRotation` _suncomponent (`KismetMathLibrary.MakeRotator` 0.0 (* _returnvalue_4 90.0)) false false)
  (bind _returnvalue_5 (`KismetMathLibrary.FClamp` (* _returnvalue_4 -1.0)))
  (`LightComponent.SetIntensity` _suncomponent (* (* _returnvalue_5 (`/Game/Data/BP_EnvironmentPhase2Data.SunIntensity` (`self.EnvironmentData`))) _returnvalue_3))
  (`SkyLightComponent.SetIntensity` (`self.SkyComponent`) (* (`KismetMathLibrary.Lerp` (`/Game/Data/BP_EnvironmentPhase2Data.NightSkyIntensity` (`self.EnvironmentData`)) (`/Game/Data/BP_EnvironmentPhase2Data.DaySkyIntensity` (`self.EnvironmentData`)) _returnvalue_5) _returnvalue_3))
  (bind _output_get_4 (set `self.CurrentFogDensity` (`KismetMathLibrary.FInterpTo` (`self.CurrentFogDensity`) (`KismetMathLibrary.SelectFloat` (`/Game/Data/BP_EnvironmentPhase2Data.StormFogDensity` (`self.EnvironmentData`)) (`KismetMathLibrary.SelectFloat` (`/Game/Data/BP_EnvironmentPhase2Data.HazeFogDensity` (`self.EnvironmentData`)) (`/Game/Data/BP_EnvironmentPhase2Data.CalmFogDensity` (`self.EnvironmentData`)) _returnvalue) _returnvalue_2) DeltaSeconds _weatherblendspeed)))
  (`ExponentialHeightFogComponent.SetFogDensity` _fogcomponent _output_get_4)
  (bind _output_get_5 (set `self.StormIntensity` (`KismetMathLibrary.FInterpTo` (`self.StormIntensity`) (`KismetMathLibrary.SelectFloat` 1.0 0.0 _returnvalue_2) DeltaSeconds _weatherblendspeed)))
  (`AudioComponent.SetVolumeMultiplier` (`self.WindAudio`) (`KismetMathLibrary.Lerp` (`/Game/Data/BP_EnvironmentPhase2Data.WindBaseVolume` (`self.EnvironmentData`)) (`/Game/Data/BP_EnvironmentPhase2Data.WindStormVolume` (`self.EnvironmentData`)) _output_get_5))
  (`ExponentialHeightFogComponent.SetFogInscatteringColor` _fogcomponent (`KismetMathLibrary.MakeColor` (* (`/Game/Data/BP_EnvironmentPhase2Data.FogRed` (`self.EnvironmentData`)) (`KismetMathLibrary.FMax` _returnvalue_5 0.015)) (* (`/Game/Data/BP_EnvironmentPhase2Data.FogGreen` (`self.EnvironmentData`)) (`KismetMathLibrary.FMax` _returnvalue_5 0.015)) (* (`/Game/Data/BP_EnvironmentPhase2Data.FogBlue` (`self.EnvironmentData`)) (`KismetMathLibrary.FMax` _returnvalue_5 0.015)) 1.0))
  (`self.OnEnvironmentChanged`))

(fn `GetEnvironmentState`
  (returns (Weather :type Integer) (TimeOfDay :type "Float (double-precision)") (StormIntensity :type "Float (double-precision)"))
  (return (`self.Weather`) (`self.TimeOfDay`) (`self.StormIntensity`)))

(fn `SetTimeOfDay`
  (params (Value :type "Float (double-precision)"))
  (set `self.TimeOfDay` (`KismetMathLibrary.FClamp` Value 0.0 1.0)))

(fn `SetWeather`
  (params (Value :type Integer))
  (bind _output_get (set `self.Weather` (`KismetMathLibrary.Clamp` Value 0 2)))
  (set `self.WeatherElapsed` 0.0)
  (set `self.WeatherStage` _output_get))

(fn `UserConstructionScript`)